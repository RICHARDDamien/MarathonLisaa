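; BP_Mirror_Preview is the preview actor for a mirror, showing whether the pose being previewed is valid.
; SetMaterial_Event switches the StaticMesh and Reflexion materials between valid and invalid looks from two inputs: length good and on the ground.
; Tick is empty, and the event binding and downward ground trace with debug prints are disconnected; a note marks logic as outdated and points to the character.
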(event Custom|SetMaterial_Event
  (params (IsLenghtGood :type Boolean) (IsOnTheGround :type Boolean))
  ;[1 1 1] Set Material
  (if (and IsLenghtGood IsOnTheGround)
    (Rendering|Material|SetMaterial (Variables|Default|GetStaticMesh) 0 "/Game/Core/Mirror/M_PrevisualisationPose.M_PrevisualisationPose")
    (else
      (Rendering|Material|SetMaterial (Variables|Default|GetStaticMesh) 0 "/Game/Core/Mirror/M_PrevisualisationPose-INVALIDE_Inst.M_PrevisualisationPose-INVALIDE_Inst"))))

(event EventTick
  (params (DeltaSeconds :type Float%20%28single-precision%29))
  ;[1 1 1] Outdated > In the chara mtf
)

(fn ConstructionScript
  (|CallParentFunction))