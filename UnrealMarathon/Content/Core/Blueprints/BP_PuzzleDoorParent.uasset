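; Parent Blueprint for a puzzle door that slides between its placed position and the second point of its spline.
; OpenDoor plays and CloseDoor reverses the SetPosition timeline, each with a mechanical sound.
; The timeline lerps both meshes to the same swept location, holding the original rotation.
; On BeginPlay it caches both endpoints and plays the opening movement if IsInTheWay is false.
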(event Custom|OpenDoor
  ;[1 1 1] PutAway
  (Audio|PlaySound2D "/Game/Core/Sound/321867__nicistarful__fast-throttle-mechanic-lever.321867__nicistarful__fast-throttle-mechanic-lever" 0.5 1.0 0.0 0 0)
  (bind _toposition (Timeline|SetPosition Play)
    (:Update
      (Transformation|SetWorldLocationAndRotation (Variables|Default|GetStaticMesh) (Math|Vector|Lerp(Vector) (Variables|Default|GetLocationA) (Variables|Default|GetLocationB) _toposition) (Variables|Default|GetOriginalRotation) true false))))

(event Custom|CloseDoor
  ;[1 1 1] PutInTheWay
  (Audio|PlaySound2D "/Game/Core/Sound/321867__nicistarful__fast-throttle-mechanic-lever.321867__nicistarful__fast-throttle-mechanic-lever" 0.5 -1.0 0.0 0 0)
  (bind _toposition (Timeline|SetPosition Reverse)
    (:Update
      (Transformation|SetWorldLocationAndRotation (Variables|Default|GetStaticMesh) (Math|Vector|Lerp(Vector) (Variables|Default|GetLocationA) (Variables|Default|GetLocationB) _toposition) (Variables|Default|GetOriginalRotation) true false))))

(event Collision|EventActorBeginOverlap
  (params (OtherActor :type Actor%20Object%20Reference)))

(event EventTick
  (params (DeltaSeconds :type Float%20%28single-precision%29)))

(event EventBeginPlay
  (Variables|Default|SetOriginalRotation (Transformation|GetWorldRotation (Variables|Default|GetStaticMesh)))
  (Variables|Default|SetLocationA (Transformation|GetWorldLocation (Variables|Default|GetStaticMesh)))
  (Variables|Default|SetLocationB (Spline|GetLocationatSplinePoint (Variables|Default|GetSpline) 1 "World"))
  (if (not (Variables|Default|GetIsInTheWay))
    (bind _toposition (Timeline|SetPosition Play)
      (:Update
        (Transformation|SetWorldLocationAndRotation (Variables|Default|GetStaticMesh) (Math|Vector|Lerp(Vector) (Variables|Default|GetLocationA) (Variables|Default|GetLocationB) _toposition) (Variables|Default|GetOriginalRotation) true false)))))

(fn ConstructionScript)