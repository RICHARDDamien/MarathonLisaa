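; Pressure plate actor that drives a list of puzzle doors when something overlaps it.
; Overlap sinks the mesh and opens or closes each door by its IsInTheWay flag; leaving reverses both.
; While pressed, a looping timer box-traces from the plate and resets it if the hit two-world interactive is not visible.
; BeginPlay only casts the doors, as the IsInTheWay assignment from ListOfIntheway is disconnected.
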(event Custom|CheckUp
  (bind _staticmesh (Variables|Default|GetStaticMesh))
  (bind _returnvalue (Transformation|GetWorldLocation _staticmesh))
  (bind _outhit (Collision|BoxTraceByChannel _returnvalue (* _returnvalue (* (Math|Vector|GetUpVector _staticmesh) 2e+01)) "5.000000,5.000000,5.000000" "0, 0, 0" "TraceTypeQuery1" false 0 "ForDuration"))
  (bind _asbase_two_world_interactive (Utilities|Casting|CastToBase_Two_World_Interactive (.hitactor _outhit)))
  (if (not (Variables|/Game/Core/TwoWorldsObject/Base_Two_World_Interactive.Base_Two_World_Interactive_C|GetVisible? _asbase_two_world_interactive))
    (CallFunction|ResetPres)))

(event Custom|ResetPres
  (for _array_element (Variables|Default|Getlist%20of%20Element)
    (bind _asbp_puzzle_door_parent (Utilities|Casting|CastToBP_PuzzleDoorParent _array_element))
    (if (Variables|/Game/Core/Blueprints/BP_PuzzleDoorParent.BP_PuzzleDoorParent_C|GetIsInTheWay _asbp_puzzle_door_parent)
      (Default|CloseDoor _asbp_puzzle_door_parent)
      (else
        (Default|OpenDoor _asbp_puzzle_door_parent)))
    (Components|MoveComponentTo (Variables|Default|GetStaticMesh) "0, 0, 0" "0, 0, 0" false false 0.4 false)
    (Utilities|Time|ClearandInvalidateTimerbyHandle (stale Collision|EventActorBeginOverlap _returnvalue))))

(event Collision|EventActorBeginOverlap
  (params (OtherActor :type Actor%20Object%20Reference))
  (for _array_element (Variables|Default|Getlist%20of%20Element)
    (bind _asbp_puzzle_door_parent (Utilities|Casting|CastToBP_PuzzleDoorParent _array_element))
    (if (Variables|/Game/Core/Blueprints/BP_PuzzleDoorParent.BP_PuzzleDoorParent_C|GetIsInTheWay _asbp_puzzle_door_parent)
      (Default|OpenDoor _asbp_puzzle_door_parent)
      (else
        (Default|CloseDoor _asbp_puzzle_door_parent)))
    (Components|MoveComponentTo (Variables|Default|GetStaticMesh) "0, 0,-20.000000" "0, 0, 0" false false 0.4 false)
    (bind _returnvalue (Utilities|Time|SetTimerbyEvent (delegate Custom|CheckUp) 0.5 true))))

(event Collision|EventActorEndOverlap
  (params (OtherActor :type Actor%20Object%20Reference))
  (for _array_element (Variables|Default|Getlist%20of%20Element)
    (bind _asbp_puzzle_door_parent (Utilities|Casting|CastToBP_PuzzleDoorParent _array_element))
    (if (Variables|/Game/Core/Blueprints/BP_PuzzleDoorParent.BP_PuzzleDoorParent_C|GetIsInTheWay _asbp_puzzle_door_parent)
      (Default|CloseDoor _asbp_puzzle_door_parent)
      (else
        (Default|OpenDoor _asbp_puzzle_door_parent)))
    (Components|MoveComponentTo (Variables|Default|GetStaticMesh) "0, 0, 0" "0, 0, 0" false false 0.4 false)
    (Utilities|Time|ClearandInvalidateTimerbyHandle (stale Collision|EventActorBeginOverlap _returnvalue))))

(event EventTick
  (params (DeltaSeconds :type Float%20%28single-precision%29)))

(event EventBeginPlay
  (for (_array_element _array_index) (Variables|Default|Getlist%20of%20Element)
    (bind _asbp_puzzle_door_parent (Utilities|Casting|CastToBP_PuzzleDoorParent _array_element))))

(fn ConstructionScript)