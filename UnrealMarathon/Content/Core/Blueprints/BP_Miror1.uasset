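; BP_Miror1 is a mirror actor that scans with invisible line traces and enables player input when BP_Chara enters its Box.
; Each Tick casts a ring of Visibility traces from View, cycling the pitch to sweep a cone, but ignores the hits.
; The BeginPlay looping timer calls an empty event.
; Logic for tracking seen objects and showing or hiding elements through command objects is disconnected and never runs.
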(event OnComponentBeginOverlap(Box)
  (params (OverlappedComponent :type Primitive%20Component%20Object%20Reference) (OtherActor :type Actor%20Object%20Reference) (OtherComp :type Primitive%20Component%20Object%20Reference) (OtherBodyIndex :type Integer) (bFromSweep :type Boolean) (SweepResult :type Hit%20Result%20Structure%20%28by%20ref%29))
  (Utilities|Casting|CastToBP_Chara OtherActor)
  (Input|EnableInput (Game|GetPlayerController 0)))

(event Custom|CustomEvent_0)

(event EventBeginPlay
  (Utilities|Time|SetTimerbyEvent (delegate Custom|CustomEvent_0) 3.0 true))

(event EventTick
  (params (DeltaSeconds :type Float%20%28single-precision%29))
  (bind _view (Variables|Default|GetView))
  (bind _returnvalue (Transformation|GetWorldLocation _view))
  (Math|Float|IncrementFloat (Variables|Default|GetZ_Value)
    (:%20%20
      (if (>= (Variables|Default|GetActual_Angle) 1.0)
        (Variables|Default|SetActual_Angle 0.0)
        (else
          (Variables|Default|SetActual_Angle (+ (Variables|Default|GetActual_Angle) 0.1))))
      (for _index (range 0 (- (Variables|Detection|GetTraceCount) 1))
        (bind _output_get (Variables|Detection|SetCurrent_Trace_Step _index))
        (Collision|LineTraceByChannel _returnvalue (+ _returnvalue (Math|Vector|RotateVector (* (Math|Vector|RotateVector (Transformation|GetActorForwardVector) (Math|Rotator|MakeRotator 0.0 (Math|Float|Lerp 45.0 9e+01 (Variables|Default|GetActual_Angle)) (* _output_get (/ 3.6e+02 (Math|Conversions|ToFloat(Integer) (Variables|Detection|GetTraceCount)))))) (Variables|Detection|GetCheckRange)) (Math|Rotator|MakeRotator 0.0 -9e+01 0.0))) "TraceTypeQuery1" false 0 "None")))))

(event Input|KeyboardEvents|E
  (params (Key :type Key%20Structure :default "None")))

(fn ConstructionScript)