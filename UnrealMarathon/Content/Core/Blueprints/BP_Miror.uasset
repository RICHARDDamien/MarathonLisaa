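; Mirror actor (WIP) that reveals or hides two-world IRL and Mirror objects caught in its field of view.
; Tick fires batched line traces from Reflexion, sweeping yaw and stepping height to scan the area.
; Each newly hit object toggles visibility via Show/Hide command objects; E or Reset_PickUp restores IRL objects, hides Mirror ones and clears tracking.
; Vertex, box and cone trace detection experiments remain disconnected.
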(event Custom|CustomEvent_0
  (bind _reflexion (Variables|Default|GetReflexion))
  (bind _returnvalue (Transformation|GetWorldLocation _reflexion))
  (Collision|LineTraceByChannel _returnvalue (+ _returnvalue (* (Transformation|GetActorForwardVector) (Variables|Detection|GetCheckRange))) "TraceTypeQuery1" false 0 "ForDuration" true "(R=1.000000,G=0.827781,B=0.000000,A=1.000000)"))

(event Custom|Reset_PickUp
  (for _array_element (Variables|Default|GetObject_In_Vision)
    (bind _asirl_object (Utilities|Casting|CastToIRL_Object _array_element)
      (:then
        ;[1 1 1] Use To Show Element
        (bind _returnvalue (Game|ConstructObjectfromClass _asirl_object "/Game/Core/Command/ShowElement_Command.ShowElement_Command_C" _asirl_object))
        (Default|ShowElement _returnvalue)
        (Audio|PlaySound2D 0 1.0 1.0 0.0 0 0))
      (:CastFailed
        (bind _asmirror_object (Utilities|Casting|CastToMirror_Object _array_element))
        ;[1 1 1] Use To Hide Element
        (bind _returnvalue_2 (Game|ConstructObjectfromClass _asmirror_object "/Game/Core/Command/HideElement_Command.HideElement_Command_C" _asmirror_object))
        (Default|HideElement _returnvalue_2)
        (Audio|PlaySound2D 0 1.0 1.0 0.0 0 0))))
  (Utilities|Array|Clear (Variables|Default|GetObject_In_Vision))
  (Utilities|Array|Clear (Variables|Default|GetInteractive_In_Scene)))

(event Custom|CustomEvent_1
  ;[1 0 0.639] Autre manière Faire Mirror with vertex WIP
)

(event EventBeginPlay
  (Variables|Default|SetZ_Value (Variables|Default|GetMaxZValue))
  (bind _outactors (Actor|GetAllActorsOfClass "/Game/Core/TwoWorldsObject/Base_Two_World_Interactive.Base_Two_World_Interactive_C"))
  (Variables|Default|SetInteractive_In_Scene _outactors))

(event EventTick
  (params (DeltaSeconds :type Float%20%28single-precision%29))
  (bind _reflexion (Variables|Default|GetReflexion))
  (bind _returnvalue (Transformation|GetWorldLocation _reflexion))
  (for _index (range 0 90)
    (if (>= (Variables|Default|GetActual_Angle) 1.0)
      (Variables|Default|SetActual_Angle 0.0)
      (Variables|Default|SetZ_Value (- (Variables|Default|GetZ_Value) 1.5e+02))
      (if (> (Variables|Default|GetZ_Value) (Variables|Default|GetminZValue))
        _
        (else
          (Variables|Default|SetZ_Value (Variables|Default|GetMaxZValue))
          (Development|PrintString (Utilities|String|Append "seconds : " (Utilities|String|ToString(Float) (Utilities|Time|GetTimeSeconds))))))
      (else
        (Variables|Default|SetActual_Angle (+ (Variables|Default|GetActual_Angle) 0.033))))
    (bind _outhit (Collision|LineTraceByChannel _returnvalue (Math|Vector|MakeVector (.x (+ _returnvalue (* (Math|Vector|RotateVector (Transformation|GetActorForwardVector) (Math|Rotator|MakeRotator 0.0 0.0 (Math|Float|Lerp 45.0 -45.0 (Variables|Default|GetActual_Angle)))) (Variables|Detection|GetCheckRange)))) (.y (+ _returnvalue (* (Math|Vector|RotateVector (Transformation|GetActorForwardVector) (Math|Rotator|MakeRotator 0.0 0.0 (Math|Float|Lerp 45.0 -45.0 (Variables|Default|GetActual_Angle)))) (Variables|Detection|GetCheckRange)))) (+ (.z (+ _returnvalue (* (Math|Vector|RotateVector (Transformation|GetActorForwardVector) (Math|Rotator|MakeRotator 0.0 0.0 (Math|Float|Lerp 45.0 -45.0 (Variables|Default|GetActual_Angle)))) (Variables|Detection|GetCheckRange)))) (Variables|Default|GetZ_Value))) "TraceTypeQuery1" false 0 "ForOneFrame"))
    (bind _asbase_two_world_interactive (Utilities|Casting|CastToBase_Two_World_Interactive (.hitactor _outhit)))
    (if (not (Utilities|Array|ContainsItem (Variables|Default|GetObject_In_Vision) _asbase_two_world_interactive))
      (Utilities|Array|Add (Variables|Default|GetObject_In_Vision) _asbase_two_world_interactive)
      (bind _asirl_object (Utilities|Casting|CastToIRL_Object _asbase_two_world_interactive)
        (:then
          (Utilities|Array|Add (Variables|Default|GetIRL_Object_List) _asirl_object)
          (if (not (Variables|/Game/Core/TwoWorldsObject/Base_Two_World_Interactive.Base_Two_World_Interactive_C|GetVisible? _asirl_object))
            ;[1 1 1] Use To Show Element
            (bind _returnvalue_2 (Game|ConstructObjectfromClass _asirl_object "/Game/Core/Command/ShowElement_Command.ShowElement_Command_C" _asirl_object))
            (Default|ShowElement _returnvalue_2)
            (Audio|PlaySound2D 0 1.0 1.0 0.0 0 0)
            (Development|PrintString (Utilities|GetDisplayName _asirl_object))
            (else
              ;[1 1 1] Use To Hide Element
              (bind _returnvalue_3 (Game|ConstructObjectfromClass _asirl_object "/Game/Core/Command/HideElement_Command.HideElement_Command_C" _asirl_object))
              (Default|HideElement _returnvalue_3)
              (Audio|PlaySound2D 0 1.0 1.0 0.0 0 0)
              (Class|SceneCaptureComponent|HideActorComponents (Variables|Default|GetView) 0 true))))
        (:CastFailed
          (bind _asmirror_object (Utilities|Casting|CastToMirror_Object _asbase_two_world_interactive))
          (Utilities|Array|Add (Variables|Default|GetMirror_Object_List) _asmirror_object)
          (if (not (Variables|/Game/Core/TwoWorldsObject/Base_Two_World_Interactive.Base_Two_World_Interactive_C|GetVisible? _asmirror_object))
            ;[1 1 1] Use To Show Element
            (bind _returnvalue_4 (Game|ConstructObjectfromClass _asmirror_object "/Game/Core/Command/ShowElement_Command.ShowElement_Command_C" _asmirror_object))
            (Default|ShowElement _returnvalue_4)
            (Audio|PlaySound2D 0 1.0 1.0 0.0 0 0)
            (else
              ;[1 1 1] Use To Hide Element
              (bind _returnvalue_5 (Game|ConstructObjectfromClass _asmirror_object "/Game/Core/Command/HideElement_Command.HideElement_Command_C" _asmirror_object))
              (Default|HideElement _returnvalue_5)
              (Audio|PlaySound2D 0 1.0 1.0 0.0 0 0))))))))

(event Input|KeyboardEvents|E
  (params (Key :type Key%20Structure :default "None"))
  (:Pressed
    (for _array_element (Variables|Default|GetIRL_Object_List)
      (Class|ICommand|ShowElement(Message) _array_element))
    (for _array_element_2 (Variables|Default|GetMirror_Object_List)
      (Class|ICommand|HideElement(Message) _array_element_2))
    (Utilities|Array|Clear (Variables|Default|GetObject_In_Vision))
    (Utilities|Array|Clear (Variables|Default|GetIRL_Object_List))
    (Utilities|Array|Clear (Variables|Default|GetMirror_Object_List))))

(fn ConstructionScript)

(fn DetectVertex
  (params (StaticMesh :type Base%20Two%20World%20Interactive%20Object%20Reference))
  (bind _vertices (Class|KismetProceduralMeshLibrary|GetSectionfromStaticMesh (Variables|/Script/Engine.StaticMeshComponent|GetStaticMesh (Variables|/Game/Core/TwoWorldsObject/Base_Two_World_Interactive.Base_Two_World_Interactive_C|GetStaticMesh StaticMesh))))
  (return _vertices))