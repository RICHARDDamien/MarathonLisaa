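; Test player character, marked OLD, that previews and places mirrors when it has one.
; Left click spawns a preview attached to RefMirror, then places BP_Miror if ground is below; right click cancels.
; Mouse wheel yaws the preview, with near-sideways angles lengthening the clearance check.
; Tick line-traces forward from the capsule using spring arm length to update preview validity, though placement only tests for ground.
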(event Collision|EventActorBeginOverlap
  (params (OtherActor :type Actor%20Object%20Reference)))

(event EventBeginPlay
  (Development|PrintString (Utilities|GetDisplayName self)))

(event EventTick
  (params (DeltaSeconds :type Float%20%28single-precision%29))
  (bind _capsulecomponent (Variables|Default|GetCapsuleComponent))
  (bind _returnvalue (Transformation|GetWorldTransform _capsulecomponent))
  (if (Variables|Default|GetIsMirrorPreview_0)
    ;[1 1 1] Check Distance Mrroir
    (Utilities|FlowControl|Sequence
      (:then_0
        (if (Variables|Default|GetIsLenghtGood_0)
          (Variables|Default|SetLenghtSecurity_0 1.8)
          (else
            (Variables|Default|SetLenghtSecurity_0 1.5))))
      (:then_1
        (bind _outhit (Collision|LineTraceByChannel (.location _returnvalue) (+ (.location _returnvalue) (* (Math|Vector|GetForwardVector (.rotation _returnvalue)) (* (Variables|/Script/Engine.SpringArmComponent|GetTargetArmLength (Variables|Default|GetSpringArm_Ref-Mirror)) (Variables|Default|GetLenghtSecurity_0)))) "TraceTypeQuery1" false 0 "ForDuration" true "(R=0.222160,G=0.735840,B=1.000000,A=1.000000)" "(R=1.000000,G=0.000000,B=0.039356,A=1.000000)" 0.0))
        (if (.bBlockingHit (Collision|BreakHitResult _outhit))
          (Default|SetMaterialEvent (Variables|Default|GetRef-MirrorPreview_0) false false)
          (Development|PrintString "Lenght is : BAD" true true "(R=1.000000,G=0.000000,B=0.215960,A=1.000000)" 0.0)
          (else
            (Default|SetMaterialEvent (Variables|Default|GetRef-MirrorPreview_0) false false true)
            (Development|PrintString "Lenght is : GOOD" true true "(R=0.000000,G=0.660000,B=1.000000,A=1.000000)" 0.0)))))))

(event Input|MouseEvents|MouseWheelAxis
  (params (AxisValue :type Float%20%28single-precision%29))
  (bind _ref_mirror (Variables|Default|GetRef-Mirror))
  (bind _relativerotation (Variables|/Script/Engine.SceneComponent|GetRelativeRotation _ref_mirror))
  (if (Variables|Default|GetIsMirrorPreview_0)
    (Transformation|AddLocalRotation _ref_mirror (Math|Rotator|MakeRotator 0.0 0.0 (* AxisValue 1e+01)) false false)
    (if (or (and (> (.yaw _relativerotation) -1.2e+02) (< (.yaw _relativerotation) -6e+01)) (and (> (.yaw _relativerotation) 6e+01) (< (.yaw _relativerotation) 1.2e+02)))
      (Variables|Default|SetIsLenghtGood_0 true)
      (else
        (Variables|Default|SetIsLenghtGood_0 false)))))

(event Input|MouseEvents|RightMouseButton
  (params (Key :type Key%20Structure :default "None"))
  (:Pressed
    ;[1 1 1] Is Preview Shown?
    (Utilities|IsValid (Variables|Default|GetRef-MirrorPreview_0)
      (:Is%20Valid
        (Variables|Default|SetIsMirrorPreview_0 false)
        ;[1 1 1] Destroy Preview (Retour vue basique)
        (Actor|DestroyActor (Variables|Default|GetRef-MirrorPreview_0))
        (Development|PrintString "MirrorPreview Destroy"))
      (:Is%20Not%20Valid
        (Development|PrintString "Mirror Zoom ?")))))

(event Input|MouseEvents|LeftMouseButton
  (params (Key :type Key%20Structure :default "None"))
  (:Pressed
    (if (Variables|Default|GetHasMiror_0)
      ;[1 1 1] Is Preview Shown?
      (Utilities|IsValid (Variables|Default|GetRef-MirrorPreview_0)
        (:Is%20Valid
          (Development|PrintString "Pose Miroir / Destroy Preview")
          (if (Variables|/Game/Core/Mirror/BP_Mirror_Preview.BP_Mirror_Preview_C|GetIsGroundBelow (Variables|Default|GetRef-MirrorPreview_0))
            (Game|SpawnActorfromClass "/Game/Core/Blueprints/BP_Miror.BP_Miror_C" (Transformation|GetActorTransform (Variables|Default|GetRef-MirrorPreview_0)) "Undefined" 0 0)
            (Variables|Default|SetIsMirrorPreview_0 false)
            (Actor|DestroyActor (Variables|Default|GetRef-MirrorPreview_0))))
        (:Is%20Not%20Valid
          (Variables|Default|SetIsMirrorPreview_0 true)
          (bind _returnvalue (Game|SpawnActorfromClass "/Game/Core/Mirror/BP_Mirror_Preview.BP_Mirror_Preview_C" (Math|Transform|MakeTransform "1.000000,1.000000,1.000000" "0, 0, 0" "1.000000,1.000000,1.000000") "Undefined" 0 0))
          (bind _output_get (Variables|Default|SetRef-MirrorPreview_0 _returnvalue))
          (Transformation|AttachComponentToComponent _output_get (Variables|Default|GetRef-Mirror) "None" "KeepRelative" "KeepRelative" "KeepRelative" true)
          (Development|PrintString "MirrorPreview Spawn"))))))

(fn ConstructionScript
  (|CallParentFunction))