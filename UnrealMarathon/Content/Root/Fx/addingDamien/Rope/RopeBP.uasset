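; Rope actor Blueprint that builds a rope from spline mesh segments along its Spline in the construction script.
; It divides the spline length by a Section length scaled by actor X scale and adds one Z-forward spline mesh per step.
; Each segment takes local positions and tangents from the spline, with tangents clamped to the section length.
; The event graph has no active logic.
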(event EventBeginPlay)

(event Collision|EventActorBeginOverlap
  (params (OtherActor :type Actor%20Object%20Reference)))

(event EventTick
  (params (DeltaSeconds :type Float%20%28single-precision%29)))

(fn ConstructionScript
  (bind _spline (Variables|Default|GetSpline))
  (bind _spline_2 (Variables|Default|GetSpline))
  (Variables|Default|Setsection (* (Variables|Default|Getsection) (.x (Transformation|GetActorScale3D))))
  (for _index (range 0 (Math|Float|Truncate (/ (Spline|GetSplineLength (Variables|Default|GetSpline)) (Variables|Default|Getsection))))
    (bind _returnvalue (AddComponent|AddSplineMeshComponent false))
    (SplineMesh|SetForwardAxis _returnvalue "Z" true)
    (SplineMesh|SetStartandEnd _returnvalue (Spline|GetLocationatDistanceAlongSpline _spline_2 (* _index (Variables|Default|Getsection)) "Local") (Math|Vector|ClampVectorSize (Spline|GetTangentatDistanceAlongSpline _spline_2 (* _index (Variables|Default|Getsection)) "Local") 0.0 (Variables|Default|Getsection)) (Spline|GetLocationatDistanceAlongSpline _spline (* (+ _index 1) (Variables|Default|Getsection)) "Local") (Math|Vector|ClampVectorSize (Spline|GetTangentatDistanceAlongSpline _spline (* (+ _index 1) (Variables|Default|Getsection)) "Local") 0.0 (Variables|Default|Getsection)) true :!class /Script/Engine.SplineMeshComponent)))